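; Zend is a player-controlled character Blueprint with movement, camera look, jump, dash and a sword light attack.
; Axis inputs drive control-rotation-relative movement and controller yaw and pitch.
; Attack input sets a LightAttack flag that StopAttack clears, while the Draw event sets Drawn and attaches DemonSword at a hand socket.
; Dashu input sets a Roll animation on the mesh, applies a large forward impulse and prints a debug string.
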(event Custom|Draw
  (Variables|Default|SetDrawn true)
  (Transformation|AttachComponentToComponent (Variables|Default|GetDemonSword) (Variables|Default|GetScene1) "HandR_0" "KeepRelative" "KeepRelative" "KeepWorld" false)
  (Components|MoveComponentTo 0 "0, 0, 0" "0, 0, 0" false false 0.0 false))

(event Custom|StopAttack
  (Variables|Default|SetLightAttack false))

(event EventBeginPlay)

(event EventTick
  (params (DeltaSeconds :type Float%20%28single-precision%29)))

(event Collision|EventActorBeginOverlap
  (params (OtherActor :type Actor%20Object%20Reference)))

(event Input|ActionEvents|InputActionJump
  (params (Key :type Key%20Structure :default "None"))
  (:Pressed
    (Character|Jump)))

(event Input|ActionEvents|InputActionAttack
  (params (Key :type Key%20Structure :default "None"))
  (:Pressed
    (Variables|Default|SetLightAttack true)))

(event Input|ActionEvents|InputActionDashu
  (params (Key :type Key%20Structure :default "None"))
  (:Pressed
    (Components|Animation|SetAnimation (Variables|Character|GetMesh) "/Game/Models/Animations/Roll.Roll")
    (Physics|AddImpulse (Variables|Character|GetCharacterMovement) (* (Transformation|GetActorForwardVector) 7.5e+05) false)
    (Development|PrintString "Hello")))

(event Input|AxisEvents|InputAxisHortizontal
  (params (AxisValue :type Float%20%28single-precision%29))
  ;[1 1 1] Movement
  (Pawn|Input|AddMovementInput (Math|Vector|GetRightVector (Pawn|GetControlRotation :!class /Script/Engine.Pawn)) AxisValue false))

(event Input|AxisEvents|InputAxisVertical
  (params (AxisValue :type Float%20%28single-precision%29))
  ;[1 1 1] Movement
  (Pawn|Input|AddMovementInput (Math|Vector|GetForwardVector (Math|Rotator|MakeRotator 0.0 0.0 (.Yaw (Math|Rotator|BreakRotator (Pawn|GetControlRotation :!class /Script/Engine.Pawn))))) AxisValue false))

(event Input|AxisEvents|InputAxisTurnRotations
  (params (AxisValue :type Float%20%28single-precision%29))
  ;[1 1 1] CameraRotations
  (Pawn|Input|AddControllerYawInput AxisValue))

(event Input|AxisEvents|InputAxisLookUp
  (params (AxisValue :type Float%20%28single-precision%29))
  ;[1 1 1] CameraRotations
  (Pawn|Input|AddControllerPitchInput AxisValue))

(fn ConstructionScript)